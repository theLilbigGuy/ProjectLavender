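; BP_DamagableParent is a test Blueprint, named as a parent for damaging effects, that lets Niagara particles hurt the player.
; On BeginPlay it passes itself to the Niagara component's BP_CallBack variable to receive exported particle data.
; Each ParticleData callback sends player 0 a fixed damage message, regardless of particle positions.
; An unconnected loop sketches per-particle sphere traces along velocity with debug drawing, but never runs.
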(event EventBeginPlay
  (Class|NiagaraComponent|SetVariableObject (Variables|Default|GetNiagara) "BP_CallBack" self))

(event EventParticleData
  (params (Data :type Array%20of%20Basic%20Particle%20Data%20Structures) (NiagaraSystem :type Niagara%20System%20Object%20Reference))
  (Class|BPIDamagable|TakeDamage(Message) (Game|GetPlayerCharacter 0) 5.0))

(fn ConstructionScript)