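; Base interactable actor for the Dolly player, with a mesh, sphere trigger and prompt UI.
; The construction script applies mesh and UI settings from variables, but trigger setup is never called.
; Trigger overlaps add or remove the actor from BP_DollyPlayer's interactions, and ToggleUI sets prompt visibility.
; The Interactwith event calls Interact, which here only stores the interacting character.
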(event OnComponentBeginOverlap(InteractionTrigger)
  (params (OverlappedComponent :type Primitive%20Component%20Object%20Reference) (OtherActor :type Actor%20Object%20Reference) (OtherComp :type Primitive%20Component%20Object%20Reference) (OtherBodyIndex :type Integer) (bFromSweep :type Boolean) (SweepResult :type Hit%20Result%20Structure%20%28by%20ref%29))
  ;[1 1 1] Trigger Overlap
  (bind _asbp_dolly_player (Utilities|Casting|CastToBP_DollyPlayer OtherActor))
  (Default|AddInteraction _asbp_dolly_player self))

(event OnComponentEndOverlap(InteractionTrigger)
  (params (OverlappedComponent :type Primitive%20Component%20Object%20Reference) (OtherActor :type Actor%20Object%20Reference) (OtherComp :type Primitive%20Component%20Object%20Reference) (OtherBodyIndex :type Integer))
  ;[1 1 1] Trigger Overlap
  (bind _asbp_dolly_player (Utilities|Casting|CastToBP_DollyPlayer OtherActor))
  (Default|RemoveInteraction _asbp_dolly_player self))

(event EventBeginPlay
  (Development|PrintString "Hello"))

(event Collision|EventActorBeginOverlap
  (params (OtherActor :type Actor%20Object%20Reference)))

(event EventTick
  (params (DeltaSeconds :type Float%20%28single-precision%29)))

(event EventInteractwith
  (params (PlayerCharacter :type BP%20Dolly%20Player%20Object%20Reference))
  (Interact|Interact PlayerCharacter))

(fn ConstructionScript
  (Edit|SetupMesh)
  (Edit|SetupUI))

(fn SetupMesh
  ;[1 1 1] Setup Mesh
  (Components|StaticMesh|SetStaticMesh (Variables|Default|GetInteractionMesh) (Variables|Edit|GetInteractMesh))
  (Transformation|SetRelativeTransform (Variables|Default|GetInteractionMesh) (Variables|Edit|GetMeshTransform) false false))

(fn SetupTrigger
  ;[1 1 1] Setup Trigger
  (Components|Sphere|SetSphereRadius (Variables|Default|GetInteractionTrigger) (Variables|Edit|GetSphereRotation) true)
  (Transformation|SetRelativeLocation (Variables|Default|GetInteractionTrigger) (Variables|Edit|GetSphereLocation) false false))

(fn SetupUI
  ;[1 1 1] SetupUI
  (Transformation|SetRelativeLocation (Variables|Default|GetInteractUI) (Variables|Edit|GetUILocation) false false))

(fn ToggleUI
  (params (Visible :type Boolean))
  ;[1 1 1] Set Visibility
  (Rendering|SetVisibility (Variables|Default|GetInteractUI) Visible false))

(fn Interact
  (params (Character :type BP%20Dolly%20Player%20Object%20Reference))
  ;[1 1 1] Interaction
  (Variables|Default|SetInteractCharacter Character))