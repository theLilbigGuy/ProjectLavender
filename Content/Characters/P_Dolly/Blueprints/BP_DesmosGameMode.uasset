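; BP_DesmosGameMode is a game mode that creates Dolly's HUD and tracks the state of the support menus for gate skills and seals.
; BeginPlay adds UI_DollyHud to the viewport and sets SupportState through the off values, ending on BuffMenuOFF.
; OpenGateSkills and OpenSeals inputs, gated by CanUseSkills and CanUseKeys, use FlipFlops and switches on SupportState to toggle menu states.
; Closing seals sets GateMenuOff rather than KeyMenuOff.
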(event EventBeginPlay
  ;[1 1 1] Create Desmos HUD
  (bind _returnvalue (UserInterface|CreateWidget "/Game/Characters/P_Dolly/Blueprints/UI/UI_DollyHud.UI_DollyHud_C"))
  (bind _output_get (Variables|Default|SetDollyHUD _returnvalue))
  (UserInterface|Viewport|AddtoViewport _output_get 0)
  ;[1 1 1] Set Support States To OFF
  (Variables|States|SetSupportState "NewEnumerator2")
  (Variables|States|SetSupportState "NewEnumerator3")
  (Variables|States|SetSupportState "NewEnumerator5")
  (Variables|States|SetSupportState "NewEnumerator7"))

(event EventTick
  (params (DeltaSeconds :type Float%20%28single-precision%29)))

(event Input|ActionEvents|InputActionOpenGateSkills
  (params (Key :type Key%20Structure :default "None"))
  (:Pressed
    (if (Variables|Skills|GetCanUseSkills?)
      (Utilities|FlowControl|FlipFlop
        (:A
          (switch Utilities|FlowControl|Switch|SwitchonE_SupportState (Variables|States|GetSupportState)
            (:NewEnumerator2
              _)
            (:NewEnumerator3
              _))
          (Variables|States|SetSupportState "NewEnumerator1"))
        (:B
          (switch Utilities|FlowControl|Switch|SwitchonE_SupportState (Variables|States|GetSupportState)
            (:NewEnumerator1
              _)
            (:NewEnumerator3
              _))
          (Variables|States|SetSupportState "NewEnumerator2")))
      (else
        (Development|PrintString "GateLocked")))))

(event Input|ActionEvents|InputActionOpenSeals
  (params (Key :type Key%20Structure :default "None"))
  ;[1 1 1] Toggle Keys Menu
  (:Pressed
    (if (Variables|Skills|GetCanUseKeys?)
      (Utilities|FlowControl|FlipFlop
        (:A
          (switch Utilities|FlowControl|Switch|SwitchonE_SupportState (Variables|States|GetSupportState)
            (:NewEnumerator2
              _)
            (:NewEnumerator3
              _))
          (Variables|States|SetSupportState "NewEnumerator0")
          (Development|PrintString "SealsActive"))
        (:B
          (switch Utilities|FlowControl|Switch|SwitchonE_SupportState (Variables|States|GetSupportState)
            (:NewEnumerator2
              _)
            (:NewEnumerator0
              _))
          (Variables|States|SetSupportState "NewEnumerator2")
          (Development|PrintString "SealsInactive"))))))

(fn ConstructionScript)