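; BP_HealStation is an interactable station that heals the player when used.
; Its Interact override calls the parent, then sends a TakeDamage interface message with a negative amount, reusing the damage path for healing.
; The heal always targets player character 0, ignoring the Character passed to Interact.
; The event graph holds only disabled stub events, and construction just calls the parent.
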(event EventBeginPlay
  (|CallParentFunction) ; This node is disabled and will not be called.\nDrag off pins to build functionality.
)

(event Collision|EventActorBeginOverlap
  (params (OtherActor :type Actor%20Object%20Reference))
  (|CallParentFunction OtherActor) ; This node is disabled and will not be called.\nDrag off pins to build functionality.
)

(event EventTick
  (params (DeltaSeconds :type Float%20%28single-precision%29))
  (|CallParentFunction DeltaSeconds) ; This node is disabled and will not be called.\nDrag off pins to build functionality.
)

(fn ConstructionScript
  (|CallParentFunction))

(fn Interact
  (params (Character :type BP%20Dolly%20Player%20Object%20Reference))
  (|CallParentFunction Character)
  (Class|BPIDamagable|TakeDamage(Message) (Game|GetPlayerCharacter 0) -1e+02))