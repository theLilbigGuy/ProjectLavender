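; Dynamic camera actor that turns to face the player while it is the active view target.
; Tick calls TrackPlayerMovement, which points the actor's X axis at the player pawn's location.
; StartCamera and EndCamera overlap events are empty; logic to blend the view to this camera and back to BP_DollyPlayer, and to store a spring arm offset, is disconnected and never runs.
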(event OnComponentBeginOverlap(StartCamera)
  (params (OverlappedComponent :type Primitive%20Component%20Object%20Reference) (OtherActor :type Actor%20Object%20Reference) (OtherComp :type Primitive%20Component%20Object%20Reference) (OtherBodyIndex :type Integer) (bFromSweep :type Boolean) (SweepResult :type Hit%20Result%20Structure%20%28by%20ref%29))
  ;[1 1 1] Start Camera Track
)

(event OnComponentBeginOverlap(EndCamera)
  (params (OverlappedComponent :type Primitive%20Component%20Object%20Reference) (OtherActor :type Actor%20Object%20Reference) (OtherComp :type Primitive%20Component%20Object%20Reference) (OtherBodyIndex :type Integer) (bFromSweep :type Boolean) (SweepResult :type Hit%20Result%20Structure%20%28by%20ref%29))
  ;[1 1 1] End Camera Track
)

(event EventBeginPlay)

(event EventTick
  (params (DeltaSeconds :type Float%20%28single-precision%29))
  (if (== (Pawn|GetViewTarget (Game|GetPlayerController 0)) self)
    (CallFunction|TrackPlayerMovement 0.0)))

(fn ConstructionScript)

(fn TrackPlayerMovement
  (params (DeltaTime :type Float%20%28single-precision%29))
  (Transformation|SetActorRelativeRotation (Math|Conversions|RotationFromXVector (- (Transformation|GetActorLocation (Game|Player|GetPlayerPawn 0)) (Transformation|GetActorLocation))))
  (return "0, 0, 0"))