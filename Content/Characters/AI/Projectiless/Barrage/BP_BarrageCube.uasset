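; BP_BarrageCube is an AI barrage projectile actor that damages the player through Niagara particle callbacks.
; On BeginPlay it registers itself as the Niagara system's callback object and copies EnemyLevel into its level-up component.
; Each ParticleData event sends damage directly to player character 0 without inspecting particle contents, scaled from the current level and rounded up.
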(event EventBeginPlay
  (Class|NiagaraComponent|SetVariableObject (Variables|Default|GetNiagara) "BP_CubeCallBack" self)
  (Variables|/Game/Characters/AI/Blueprints/AIComponenents/LevelUp/BPLevelUpComponent.BPLevelUpComponent_C|SetCurrentLevel (Variables|Default|GetBPLevelUpComponent) (Variables|Default|GetEnemyLevel)))

(event Collision|EventActorBeginOverlap
  (params (OtherActor :type Actor%20Object%20Reference)))

(event EventTick
  (params (DeltaSeconds :type Float%20%28single-precision%29)))

(event EventParticleData
  (params (Data :type Array%20of%20Basic%20Particle%20Data%20Structures) (NiagaraSystem :type Niagara%20System%20Object%20Reference))
  (bind _givenda_age (CallFunction|CalculateGiveDamage))
  (Class|BPIDamagable|TakeDamage(Message) (Game|GetPlayerCharacter 0) _givenda_age))

(fn ConstructionScript)

(fn CalculateGiveDamage
  (return (Math|Conversions|ToFloat(Integer) (Math|Float|Ceil (* (Variables|/Game/Characters/AI/Blueprints/AIComponenents/LevelUp/BPLevelUpComponent.BPLevelUpComponent_C|GetCurrentLevel (Variables|Default|GetBPLevelUpComponent)) 0.2)))))