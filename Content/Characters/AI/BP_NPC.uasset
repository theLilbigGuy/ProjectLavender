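; BP_NPC is an AI NPC that carries a health component and is destroyed when interacted with.
; BeginPlay copies its max and current health into the component, and Interactwith calls OnDeath directly, bypassing health.
; The construction script clears DialougeTree on its BPC_BasicAIController.
; DecreaseHealth and Die provide one-point damage and a zero-health destroy check, but their event-graph calls never run.
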(event EventBeginPlay
  (Variables|/Game/Characters/AI/Blueprints/AIComponenents/Health/BP_HealthComponenet.BP_HealthComponenet_C|SetMaxHealth (Variables|Default|GetBP_HealthComponenet) (Variables|Default|GetMax%20Health))
  (Variables|/Game/Characters/AI/Blueprints/AIComponenents/Health/BP_HealthComponenet.BP_HealthComponenet_C|SetCurrentHealth (Variables|Default|GetBP_HealthComponenet) (Variables|Default|GetCurrent%20Health)))

(event Collision|EventActorBeginOverlap
  (params (OtherActor :type Actor%20Object%20Reference)))

(event EventTick
  (params (DeltaSeconds :type Float%20%28single-precision%29)))

(event EventInteractwith
  (params (PlayerCharacter :type BP%20Dolly%20Player%20Object%20Reference))
  (CallFunction|OnDeath))

(event EventOnDeath
  (Actor|DestroyActor))

(fn ConstructionScript
  (bind _asbpc_basic_aicontroller (Utilities|Casting|CastToBPC_BasicAIController (AI|GetAIController self)))
  (Variables|/Game/Characters/AI/Blueprints/BPC_BasicAIController.BPC_BasicAIController_C|SetDialougeTree _asbpc_basic_aicontroller 0))

(fn DecreaseHealth
  (Variables|/Game/Characters/AI/Blueprints/AIComponenents/Health/BP_HealthComponenet.BP_HealthComponenet_C|SetCurrentHealth (Variables|Default|GetBP_HealthComponenet) (- (Variables|/Game/Characters/AI/Blueprints/AIComponenents/Health/BP_HealthComponenet.BP_HealthComponenet_C|GetCurrentHealth (Variables|Default|GetBP_HealthComponenet)) 1.0)))

(fn Die
  (if (<= (Variables|/Game/Characters/AI/Blueprints/AIComponenents/Health/BP_HealthComponenet.BP_HealthComponenet_C|GetCurrentHealth (Variables|Default|GetBP_HealthComponenet)) 0.0)
    (Actor|DestroyActor)))