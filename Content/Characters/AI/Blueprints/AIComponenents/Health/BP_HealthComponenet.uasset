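; Health component for AI characters that tracks current health against a maximum.
; GetDamaged subtracts incoming damage from current health and records the amount in DamageGiven.
; Every Tick, AtMaxHealth clamps current health down to the maximum, with no lower bound or death handling.
; CheckHealth, UpdateMaxHealth and SetMaxHealth are stubs, with only disconnected, reversed damage math left in CheckHealth.
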(event EventBeginPlay)

(event EventTick
  (params (DeltaSeconds :type Float%20%28single-precision%29))
  (CallFunction|AtMaxHealth))

(fn CheckHealth
  (params (Damage :type Float%20%28single-precision%29)))

(fn UpdateMaxHealth)

(fn SetMaxHealth)

(fn GetDamaged
  (params (Damage :type Float%20%28single-precision%29))
  ;[1 1 1] Get Damaged
  (Variables|Default|SetCurrentHealth (- (Variables|Default|GetCurrentHealth) Damage))
  (Variables|Default|SetDamageGiven Damage))

(fn AtMaxHealth
  ;[1 1 1] Resest To Max Health If Over Max
  (if (> (Variables|Default|GetCurrentHealth) (Variables|Default|GetMaxHealth))
    (Variables|Default|SetCurrentHealth (Variables|Default|GetMaxHealth))))