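; Reaper AI ability Blueprint that provides a Phase Dash for its character.
; PhaseDash uses a DoOnce reset after delays as a cooldown around the Dash macro.
; Dash launches the character upward, then forward by LaunchPower, and disables capsule collision to phase through blockade damage.
; The collision re-enable call and the AirFriction velocity damping are disconnected, so collision stays off and air friction does nothing.
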(event Custom|PhaseDash
  ;[1 1 1] Dash When in Stable State
  (Utilities|FlowControl|DoOnce false :!label _label
    (:Completed
      (Utilities|Dash)
      (Utilities|FlowControl|Delay 0.4)
      (Utilities|FlowControl|Delay 0.8)
      (goto _label Reset))))

(event EventBeginPlay)

(event EventTick
  (params (DeltaSeconds :type Float%20%28single-precision%29)))

(fn AirFriction)