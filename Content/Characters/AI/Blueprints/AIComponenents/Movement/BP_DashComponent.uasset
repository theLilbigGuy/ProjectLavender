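; AI character component that provides a dash ability, hiding the mesh and temporarily changing movement.
; StartDash hides the mesh and overrides walk speed, acceleration and rotation rate on CharacterMovement.
; Helpers set a supplied timeline's play rate, derive DashSpeed as rate times distance, and spawn an attached Niagara dash effect.
; Separate functions restore movement values and mesh visibility, but nothing in this file calls them.
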(event Custom|StartDash
  (CallFunction|HideMesh)
  (CallFunction|SetCharacterMovement))

(event EventBeginPlay)

(event EventTick
  (params (DeltaSeconds :type Float%20%28single-precision%29)))

(fn HideMesh
  (params (Mesh :type Scene%20Component%20Object%20Reference))
  (Rendering|SetVisibility Mesh false false))

(fn SetCharacterMovement
  (params (CharacterMovement :type Character%20Movement%20Component%20Object%20Reference))
  (Variables|/Script/Engine.CharacterMovementComponent|SetMaxWalkSpeed CharacterMovement (Variables|Default|GetDashSpeed))
  (Variables|/Script/Engine.CharacterMovementComponent|SetMaxAcceleration CharacterMovement (Variables|Default|GetAcceleration))
  (Variables|/Script/Engine.CharacterMovementComponent|SetRotationRate CharacterMovement (Variables|Default|GetRotationRate)))

(fn DashRate/Distance
  (params (Timeline :type Timeline%20Component%20Object%20Reference))
  (bind _dashrate (Variables|Default|GetDashRate))
  (Components|Timeline|SetPlayRate Timeline _dashrate)
  (Variables|Default|SetDashSpeed (* _dashrate (Variables|Default|GetDashDistance))))

(fn RevertCharacterMovement
  (params (Max%20Walk%20Speed :type Float%20%28single-precision%29) (Max%20Acceleration :type Float%20%28single-precision%29) (Rotation%20Rate :type Rotator) (CharacterMovement :type Character%20Movement%20Component%20Object%20Reference))
  (Variables|/Script/Engine.CharacterMovementComponent|SetMaxWalkSpeed CharacterMovement Max%20Walk%20Speed)
  (Variables|/Script/Engine.CharacterMovementComponent|SetMaxAcceleration CharacterMovement Max%20Acceleration)
  (Variables|/Script/Engine.CharacterMovementComponent|SetRotationRate CharacterMovement Rotation%20Rate))

(fn ShowCharacter
  (params (Mesh :type Scene%20Component%20Object%20Reference))
  (Rendering|SetVisibility Mesh true false))

(fn SpawnFX
  (params (SpawnLocation :type Scene%20Component%20Object%20Reference) (Rotation%20Z%20%28Yaw%29 :type Float%20%28single-precision%29))
  (bind _returnvalue (Niagara|SpawnSystemAttached "/Game/FX/SpiritualEffects/Movement/Dash/VFX_Dash_Normal.VFX_Dash_Normal" SpawnLocation "None" (Transformation|GetWorldLocation SpawnLocation) (Math|Rotator|MakeRotator 0.0 0.0 Rotation%20Z%20%28Yaw%29) "KeepWorldPosition" true))
  (Variables|Default|SetDashFX _returnvalue))