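; BP_PhasePoint is a start/end trigger pair that switches a BP_DollyPlayer into and out of its Phasing conscious state.
; Overlapping PhasePointStart changes a Stable player to Phasing and plays a 2D explosion sound.
; Overlapping PhasePointEnd returns a Phasing player to Stable.
; The actor's IsStable flag gates both triggers and flips with each change, so start and end alternate.
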(event OnComponentBeginOverlap(PhasePointStart)
  (params (OverlappedComponent :type Primitive%20Component%20Object%20Reference) (OtherActor :type Actor%20Object%20Reference) (OtherComp :type Primitive%20Component%20Object%20Reference) (OtherBodyIndex :type Integer) (bFromSweep :type Boolean) (SweepResult :type Hit%20Result%20Structure%20%28by%20ref%29))
  (if (Variables|Default|GetIsStable?)
    (bind _asbp_dolly_player (Utilities|Casting|CastToBP_DollyPlayer OtherActor))
    (switch Utilities|FlowControl|Switch|SwitchonE_ConsciousState (Variables|/Game/Characters/P_Dolly/Blueprints/BP_DollyPlayer.BP_DollyPlayer_C|GetConsciousState _asbp_dolly_player)
      (:NewEnumerator0
        (Variables|/Game/Characters/P_Dolly/Blueprints/BP_DollyPlayer.BP_DollyPlayer_C|SetConsciousState _asbp_dolly_player "NewEnumerator1")
        (Variables|Default|SetIsStable? false)
        (Audio|PlaySound2D "/Game/StarterContent/Audio/Explosion01.Explosion01" 1.0 1.0 0.0 0 0)))))

(event OnComponentBeginOverlap(PhasePointEnd)
  (params (OverlappedComponent :type Primitive%20Component%20Object%20Reference) (OtherActor :type Actor%20Object%20Reference) (OtherComp :type Primitive%20Component%20Object%20Reference) (OtherBodyIndex :type Integer) (bFromSweep :type Boolean) (SweepResult :type Hit%20Result%20Structure%20%28by%20ref%29))
  (if (not (Variables|Default|GetIsStable?))
    (bind _asbp_dolly_player (Utilities|Casting|CastToBP_DollyPlayer OtherActor))
    (switch Utilities|FlowControl|Switch|SwitchonE_ConsciousState (Variables|/Game/Characters/P_Dolly/Blueprints/BP_DollyPlayer.BP_DollyPlayer_C|GetConsciousState _asbp_dolly_player)
      (:NewEnumerator1
        (Variables|/Game/Characters/P_Dolly/Blueprints/BP_DollyPlayer.BP_DollyPlayer_C|SetConsciousState _asbp_dolly_player "NewEnumerator0")
        (Variables|Default|SetIsStable? true)))))

(event EventBeginPlay)

(event Collision|EventActorBeginOverlap
  (params (OtherActor :type Actor%20Object%20Reference)))

(event EventTick
  (params (DeltaSeconds :type Float%20%28single-precision%29)))

(fn ConstructionScript)